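; Bookcase that slides horizontally to a target location when it receives Interact, likely triggered by another object since IsInteractable returns false.
; Interact plays a world camera shake at the bookcase and starts the Movement timeline.
; Each update lerps SharedRoot's X and Y from its current position toward TargetLocation, keeping Z.
; The same update also sends an Interact message to SharedRoot.
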(event EventInteract
  (params (InteractivePlayer :type Character%20Object%20Reference))
  (bind _sharedroot (Variables|Default|GetSharedRoot))
  (bind _targetlocation (Variables|Default|GetTargetLocation))
  (bind _sharedroot_2 (Variables|Default|GetSharedRoot))
  (bind _returnvalue (Transformation|GetWorldLocation _sharedroot_2))
  (Camera|PlayWorldCameraShake "/Game/Blueprints/BP_CameraShake.BP_CameraShake_C" (Transformation|GetWorldLocation (Variables|Default|GetSharedRoot)) 0.0 5e+02)
  (bind _movementvalue (Timeline|Movement Play)
    (:Update
      (Transformation|SetWorldLocation _sharedroot (Math|Vector|MakeVector (Math|Float|Lerp (.x _returnvalue) (.x _targetlocation) (.x _movementvalue)) (Math|Float|Lerp (.y _returnvalue) (.y _targetlocation) (.y _movementvalue)) (.z _returnvalue)) false false)
      (Class|BPIInteractive|Interact(Message) _sharedroot))))

(fn ConstructionScript)

(fn IsInteractable
  (return false))